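; BP_BaseballBat is an enemy baseball bat that detects hits on the player character.
; Every tick it sphere-traces on the Camera channel between its Hit and Middle components, with debug drawing, and pushes a struck BP_ThirdPersonCharacter into a new state.
; EnableHit raises a CanHit flag for a given duration, but the tick trace does not check that flag.
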(event Custom|Enable%20Hit
  (params (Duration :type Float%20%28double-precision%29))
  (Variables|Default|SetCan%20Hit true)
  (Utilities|FlowControl|Delay Duration)
  (Variables|Default|SetCan%20Hit false))

(event EventTick
  (params (DeltaSeconds :type Float%20%28single-precision%29))
  (bind _outhits (Collision|MultiSphereTraceByChannel (Transformation|GetWorldLocation (Variables|Default|GetHit)) (Transformation|GetWorldLocation (Variables|Default|GetMiddle)) 1e+01 "TraceTypeQuery2" false 0 "ForOneFrame"))
  (for _array_element _outhits
    (bind _asbp_third_person_character (Utilities|Casting|CastToBP_ThirdPersonCharacter (.HitActor (Collision|BreakHitResult _array_element))))
    (Default|EnterState _asbp_third_person_character "NewEnumerator12")))

(fn ConstructionScript)