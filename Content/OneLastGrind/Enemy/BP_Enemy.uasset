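; BP_Enemy is an enemy actor that plays a random idle animation and reacts when its trigger is overlapped.
; On BeginPlay it picks a looping idle from IdleAnimationsList and plays it on the SKEnemy skeletal mesh.
; An Enemy_Trigger overlap plays a one-shot baseball hit animation, up or down to match the chosen idle, without filtering the overlapping actor.
; Animations play directly through PlayAnimation, and the file contains no damage or movement logic.
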(event OnComponentBeginOverlap(Enemy_Trigger)
  (params (OverlappedComponent :type Primitive%20Component%20Object%20Reference) (OtherActor :type Actor%20Object%20Reference) (OtherComp :type Primitive%20Component%20Object%20Reference) (OtherBodyIndex :type Integer) (bFromSweep :type Boolean) (SweepResult :type Hit%20Result%20Structure%20%28by%20ref%29))
  (if (== (Variables|Default|GetAnimation%20To%20Play) "/Game/OneLastGrind/Enemy/Animations/AS_BaseballUp.AS_BaseballUp")
    (Components|Animation|PlayAnimation (Variables|Default|GetSK_Enemy) "/Game/OneLastGrind/Enemy/Animations/AS_BaseballHitUp.AS_BaseballHitUp" false)
    (else
      (Components|Animation|PlayAnimation (Variables|Default|GetSK_Enemy) "/Game/OneLastGrind/Enemy/Animations/AS_BaseballHitDown.AS_BaseballHitDown" false))))

(event EventBeginPlay
  (bind _idle_animations_list (Variables|Default|GetIdle%20Animations%20List))
  (bind _output_get (Variables|Default|SetAnimation%20To%20Play (Utilities|Array|Get(acopy) _idle_animations_list (Math|Random|RandomInteger (Utilities|Array|Length _idle_animations_list)))))
  (Components|Animation|PlayAnimation (Variables|Default|GetSK_Enemy) _output_get true))

(event Collision|EventActorBeginOverlap
  (params (OtherActor :type Actor%20Object%20Reference)))

(event EventTick
  (params (DeltaSeconds :type Float%20%28single-precision%29)))

(fn ConstructionScript)