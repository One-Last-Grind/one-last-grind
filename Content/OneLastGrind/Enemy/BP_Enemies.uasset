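; Enemy that arms and swings a baseball bat when the player character comes near, spawning the bat on its hand socket at BeginPlay.
; An arming trigger stores the player and uses a forward-vector dot product to flag a left or right side.
; A swinging trigger copies that side and sets IsSwinging.
; While swinging, Tick enables bat hits unless the player's state counters the up or down swing.
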(event OnComponentBeginOverlap(Enemy_Trigger_Arming)
  (params (OverlappedComponent :type Primitive%20Component%20Object%20Reference) (OtherActor :type Actor%20Object%20Reference) (OtherComp :type Primitive%20Component%20Object%20Reference) (OtherBodyIndex :type Integer) (bFromSweep :type Boolean) (SweepResult :type Hit%20Result%20Structure%20%28by%20ref%29))
  ;[0 0 0] Trigger Arming
  ;;[0.2 1 0] Enter Trigger
  (bind _asbp_third_person_character (Utilities|Casting|CastToBP_ThirdPersonCharacter OtherActor))
  (Variables|Components|SetCharacter%20Ref _asbp_third_person_character)
  (Variables|State|SetIs%20Arming true)
  (if (> (Math|Vector|DotProduct (- (Transformation|GetActorLocation (Variables|Components|GetCharacter%20Ref)) (Transformation|GetActorLocation)) (Transformation|GetActorForwardVector)) 0.0)
    (Variables|State|SetIs%20Arming%20Left true)
    (else
      (Variables|State|SetIs%20Arming%20Right true))))

(event OnComponentEndOverlap(Enemy_Trigger_Arming)
  (params (OverlappedComponent :type Primitive%20Component%20Object%20Reference) (OtherActor :type Actor%20Object%20Reference) (OtherComp :type Primitive%20Component%20Object%20Reference) (OtherBodyIndex :type Integer))
  ;[0 0 0] Trigger Arming
  ;;[0.2 1 0] Leave Trigger
  (Utilities|Casting|CastToBP_ThirdPersonCharacter OtherActor)
  (Variables|State|SetIs%20Arming false))

(event OnComponentBeginOverlap(Enemy_Trigger_Swinging)
  (params (OverlappedComponent :type Primitive%20Component%20Object%20Reference) (OtherActor :type Actor%20Object%20Reference) (OtherComp :type Primitive%20Component%20Object%20Reference) (OtherBodyIndex :type Integer) (bFromSweep :type Boolean) (SweepResult :type Hit%20Result%20Structure%20%28by%20ref%29))
  ;[0 0 0] Trigger Swinging
  ;;[0.2 1 0] Enter Swinging
  (Utilities|Casting|CastToBP_ThirdPersonCharacter OtherActor)
  (Variables|State|SetIs%20Swinging true)
  (Variables|State|SetIs%20Swinging%20Left (Variables|State|GetIs%20Arming%20Left))
  (Variables|State|SetIs%20Swinging%20Right (Variables|State|GetIs%20Arming%20Right)))

(event OnComponentEndOverlap(Enemy_Trigger_Swinging)
  (params (OverlappedComponent :type Primitive%20Component%20Object%20Reference) (OtherActor :type Actor%20Object%20Reference) (OtherComp :type Primitive%20Component%20Object%20Reference) (OtherBodyIndex :type Integer))
  ;[0 0 0] Trigger Swinging
  ;;[0.2 1 0] Leave Swinging
  (Utilities|Casting|CastToBP_ThirdPersonCharacter OtherActor)
  (Variables|State|SetIs%20Swinging false))

(event EventBeginPlay
  ;[0 0 0] BAseball Bat
  (bind _returnvalue (Game|SpawnActorfromClass "/Game/OneLastGrind/Enemy/BP_BaseballBat.BP_BaseballBat_C" (Transformation|GetSocketTransform (Variables|Default|GetSK_Enemy) "LHS" "RTS_World") "Undefined" "MultiplyWithRoot" 0 0))
  (bind _output_get (Variables|Components|SetBat%20Ref _returnvalue))
  (Transformation|AttachComponentToComponent _output_get (Variables|Default|GetSK_Enemy) "LHS" "SnapToTarget" "SnapToTarget" "SnapToTarget" true))

(event EventTick
  (params (DeltaSeconds :type Float%20%28single-precision%29))
  ;[0 0 0] Can Hit
  (if (Variables|State|GetIs%20Swinging)
    (if (not (or (and (Variables|State|GetDown%20Swing) (Utilities|Enum|Equal(Enum) (Variables|/Game/OneLastGrind/Characters/BP_ThirdPersonCharacter.BP_ThirdPersonCharacter_C|GetCurrent%20State (Variables|Components|GetCharacter%20Ref)) "NewEnumerator7")) (and (Utilities|Enum|Equal(Enum) (Variables|/Game/OneLastGrind/Characters/BP_ThirdPersonCharacter.BP_ThirdPersonCharacter_C|GetCurrent%20State (Variables|Components|GetCharacter%20Ref)) "NewEnumerator5") (Variables|State|GetUp%20Swing))))
      (Default|EnableHit (Variables|Components|GetBat%20Ref) (Variables|Default|GetDuration)))))

(fn ConstructionScript)