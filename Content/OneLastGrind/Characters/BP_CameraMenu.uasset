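; Menu camera rig that moves a camera along a spline between designated points.
; Next/previous events pick targets using per-point stop flags; stepping back only works from the last point, returning to the first.
; A curve-driven timeline moves the camera by spline distance, easing rotation toward tangents offset by each point's direction value.
; The construction script places the camera and draws stop-colored arrows; O/P keys trigger moves in non-distribution builds.
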(event Custom|Move%20Object
  (params (Previous%20Spline%20Point :type Integer) (Next%20Spline%20Point :type Integer))
  ;[0 0 0] Move Object
  (Components|Timeline|SetPlayRate (Variables|Default|GetMove%20Object%20Timeline) (/ 1.0 (Variables|Animation|GetTime%20To%20Complete%20%28In%20Seconds%29)))
  (bind _move_track (Timeline|Move%20Object%20Timeline PlayFromStart)
    (:Update
      (bind _splinedirection (Class|MySplineActor|GetPropertyValueatSplinePoint (Math|Integer|SelectInt (Math|Float|Ceil (Class|SplineComponent|GetInputKeyValueatDistanceAlongSpline (Variables|Default|GetMySplineComponent) (Math|Float|Lerp (Spline|GetDistanceAlongSplineatSplinePoint (Variables|Default|GetMySplineComponent) Previous%20Spline%20Point) (Spline|GetDistanceAlongSplineatSplinePoint (Variables|Default|GetMySplineComponent) Next%20Spline%20Point) _move_track))) (Math|Float|Floor (Class|SplineComponent|GetInputKeyValueatDistanceAlongSpline (Variables|Default|GetMySplineComponent) (Math|Float|Lerp (Spline|GetDistanceAlongSplineatSplinePoint (Variables|Default|GetMySplineComponent) Previous%20Spline%20Point) (Spline|GetDistanceAlongSplineatSplinePoint (Variables|Default|GetMySplineComponent) Next%20Spline%20Point) _move_track))) (< Previous%20Spline%20Point Next%20Spline%20Point))))
      (Transformation|SetWorldTransform (Variables|Default|GetCamera) (Math|Transform|MakeTransform (Spline|GetLocationatDistanceAlongSpline (Variables|Default|GetMySplineComponent) (Math|Float|Lerp (Spline|GetDistanceAlongSplineatSplinePoint (Variables|Default|GetMySplineComponent) Previous%20Spline%20Point) (Spline|GetDistanceAlongSplineatSplinePoint (Variables|Default|GetMySplineComponent) Next%20Spline%20Point) _move_track) "World") (Math|Interpolation|RInterpTo (Transformation|GetWorldRotation (Variables|Default|GetCamera)) (Math|Rotator|MakeRotator (.roll (Math|Rotator|MakeRotfromX (Spline|GetTangentatSplinePoint (Variables|Default|GetMySplineComponent) (Math|Integer|SelectInt (Math|Float|Ceil (Class|SplineComponent|GetInputKeyValueatDistanceAlongSpline (Variables|Default|GetMySplineComponent) (Math|Float|Lerp (Spline|GetDistanceAlongSplineatSplinePoint (Variables|Default|GetMySplineComponent) Previous%20Spline%20Point) (Spline|GetDistanceAlongSplineatSplinePoint (Variables|Default|GetMySplineComponent) Next%20Spline%20Point) _move_track))) (Math|Float|Floor (Class|SplineComponent|GetInputKeyValueatDistanceAlongSpline (Variables|Default|GetMySplineComponent) (Math|Float|Lerp (Spline|GetDistanceAlongSplineatSplinePoint (Variables|Default|GetMySplineComponent) Previous%20Spline%20Point) (Spline|GetDistanceAlongSplineatSplinePoint (Variables|Default|GetMySplineComponent) Next%20Spline%20Point) _move_track))) (< Previous%20Spline%20Point Next%20Spline%20Point)) "World"))) (.pitch (Math|Rotator|MakeRotfromX (Spline|GetTangentatSplinePoint (Variables|Default|GetMySplineComponent) (Math|Integer|SelectInt (Math|Float|Ceil (Class|SplineComponent|GetInputKeyValueatDistanceAlongSpline (Variables|Default|GetMySplineComponent) (Math|Float|Lerp (Spline|GetDistanceAlongSplineatSplinePoint (Variables|Default|GetMySplineComponent) Previous%20Spline%20Point) (Spline|GetDistanceAlongSplineatSplinePoint (Variables|Default|GetMySplineComponent) Next%20Spline%20Point) _move_track))) (Math|Float|Floor (Class|SplineComponent|GetInputKeyValueatDistanceAlongSpline (Variables|Default|GetMySplineComponent) (Math|Float|Lerp (Spline|GetDistanceAlongSplineatSplinePoint (Variables|Default|GetMySplineComponent) Previous%20Spline%20Point) (Spline|GetDistanceAlongSplineatSplinePoint (Variables|Default|GetMySplineComponent) Next%20Spline%20Point) _move_track))) (< Previous%20Spline%20Point Next%20Spline%20Point)) "World"))) (+ (* _splinedirection 90) (.yaw (Math|Rotator|MakeRotfromX (Spline|GetTangentatSplinePoint (Variables|Default|GetMySplineComponent) (Math|Integer|SelectInt (Math|Float|Ceil (Class|SplineComponent|GetInputKeyValueatDistanceAlongSpline (Variables|Default|GetMySplineComponent) (Math|Float|Lerp (Spline|GetDistanceAlongSplineatSplinePoint (Variables|Default|GetMySplineComponent) Previous%20Spline%20Point) (Spline|GetDistanceAlongSplineatSplinePoint (Variables|Default|GetMySplineComponent) Next%20Spline%20Point) _move_track))) (Math|Float|Floor (Class|SplineComponent|GetInputKeyValueatDistanceAlongSpline (Variables|Default|GetMySplineComponent) (Math|Float|Lerp (Spline|GetDistanceAlongSplineatSplinePoint (Variables|Default|GetMySplineComponent) Previous%20Spline%20Point) (Spline|GetDistanceAlongSplineatSplinePoint (Variables|Default|GetMySplineComponent) Next%20Spline%20Point) _move_track))) (< Previous%20Spline%20Point Next%20Spline%20Point)) "World"))))) (Utilities|Time|GetWorldDeltaSeconds) 1.0) "1.000000,1.000000,1.000000") false false))))

(event Custom|Set%20Previous%20Point
  (bind _current_spline_point (Variables|Spline|GetCurrent%20Spline%20Point))
  ;[0 0 0] Set Previous Point
  (bind _next_spline_point (CallFunction|GetPreviousPoint _current_spline_point))
  (if (!= _next_spline_point _current_spline_point)
    (CallFunction|SetatPoint _next_spline_point)))

(event Custom|Set%20Next%20Point
  (bind _current_spline_point (Variables|Spline|GetCurrent%20Spline%20Point))
  ;[0 0 0] Set Next Point
  (bind _next_spline_point (CallFunction|GetNextPoint _current_spline_point true))
  (if (!= _next_spline_point _current_spline_point)
    (CallFunction|SetatPoint _next_spline_point)))

(event EventBeginPlay
  ;[0 0 0] Begin Play
  (Class|TimelineComponent|SetFloatCurve (Variables|Default|GetMove%20Object%20Timeline) (Variables|Animation|GetCamera%20Speed%20Curve) "Move Track"))

(event Input|KeyboardEvents|O
  (params (Key :type Key%20Structure :default "None"))
  (:Released
    (if (not (Class|KismetSystemLibrary|IsPackagedforDistribution))
      (CallFunction|SetPreviousPoint))))

(event Input|KeyboardEvents|P
  (params (Key :type Key%20Structure :default "None"))
  (:Released
    (if (not (Class|KismetSystemLibrary|IsPackagedforDistribution))
      (CallFunction|SetNextPoint))))

(fn ConstructionScript
  (bind _mysplinecomponent (Variables|Default|GetMySplineComponent))
  (bind _returnvalue (Spline|GetNumberOfSplinePoints _mysplinecomponent))
  (bind _returnvalue_2 (- _returnvalue 1))
  (bind _output_get (Variables|Spline|SetStart%20Spline%20Point (Math|Integer|SelectInt (Math|Integer|SelectInt _returnvalue_2 (Variables|Spline|GetStart%20Spline%20Point) (> (Variables|Spline|GetStart%20Spline%20Point) _returnvalue_2)) 0 (> (Math|Integer|SelectInt _returnvalue_2 (Variables|Spline|GetStart%20Spline%20Point) (> (Variables|Spline|GetStart%20Spline%20Point) _returnvalue_2)) 0))))
  (bind _rotator (CallFunction|GetRotatorfromSplineTangeantwithPointIndex _output_get))
  (bind _splinedirection (Class|MySplineActor|GetPropertyValueatSplinePoint _output_get))
  (Transformation|SetWorldLocationAndRotation (Variables|Default|GetCamera) (Spline|GetLocationatSplinePoint (Variables|Default|GetMySplineComponent) _output_get "World") (Math|Rotator|MakeRotator (.roll _rotator) (.pitch _rotator) (+ (* _splinedirection 90) (.yaw _rotator) 9e+01)) false false)
  (Variables|Spline|SetCurrent%20Spline%20Point (Variables|Spline|GetStart%20Spline%20Point))
  (bind _spline_points_count (CallFunction|GetSplinePointCount))
  (for _index (range 0 (- _spline_points_count 1))
    (bind (_isstoppoint _splinedirection_2) (Class|MySplineActor|GetPropertyValueatSplinePoint _index))
    (Development|PrintString (Utilities|String|ToString(Integer) _splinedirection_2))
    (bind _rotator_2 (CallFunction|GetRotatorfromSplineTangeantwithPointIndex _index))
    (bind _returnvalue_3 (AddComponent|AddArrowComponent false (Math|Transform|MakeTransform (.position (Spline|GetSplinePointAt (Variables|Default|GetMySplineComponent) _index "World")) (Math|Rotator|MakeRotator 0.0 (.roll (.rotation (Spline|GetSplinePointAt (Variables|Default|GetMySplineComponent) _index "World"))) (+ (- (.yaw _rotator_2) 9e+01) (* 90 _splinedirection_2))) "1.000000,1.000000,1.000000")))
    (Transformation|AttachComponentToComponent _returnvalue_3 0 "None" "KeepWorld" "KeepRelative" "KeepWorld" true)
    (Components|Arrow|SetArrowColor(LinearColor) _returnvalue_3 (Math|Color|SelectColor "(R=1.000000,G=0.000000,B=0.030209,A=1.000000)" "(R=0.060360,G=1.000000,B=0.000000,A=1.000000)" (== _isstoppoint 1)))))

(fn SetatPoint
  (params (Spline%20Point :type Integer))
  (bind _spline_points_count (CallFunction|GetSplinePointCount))
  (if (not (> Spline%20Point (- _spline_points_count 1)))
    (bind _output_get (LocalVariables|SetSave%20Spline%20Point (Variables|Spline|GetCurrent%20Spline%20Point)))
    (bind _output_get_2 (Variables|Spline|SetCurrent%20Spline%20Point Spline%20Point))
    (CallFunction|MoveObject _output_get _output_get_2)))

(fn GetSplinePointCount
  (return (Spline|GetNumberOfSplinePoints (Variables|Default|GetMySplineComponent))))

(fn FindDistanceAlongSplineClosesttoWorldLocation
  (params (Location :type Vector) (Spline :type Spline%20Component%20Object%20Reference))
  (bind _returnvalue (Class|SplineComponent|FindInputKeyClosesttoWorldLocation Spline Location))
  (bind _returnvalue_2 (Math|Float|Truncate _returnvalue))
  (bind _returnvalue_3 (Spline|GetDistanceAlongSplineatSplinePoint Spline _returnvalue_2))
  (return (+ _returnvalue_3 (* (- (Spline|GetDistanceAlongSplineatSplinePoint Spline (Math|Float|Truncate (+ _returnvalue 1.0))) _returnvalue_3) (- _returnvalue _returnvalue_2)))))

(fn GetRotatorfromSplineTangeantwithDistance
  (params (Distance :type Float%20%28double-precision%29))
  (bind _mysplinecomponent (Variables|Default|GetMySplineComponent))
  (bind _returnvalue (Spline|GetTangentatDistanceAlongSpline _mysplinecomponent Distance "World"))
  (bind _returnvalue_2 (Math|Conversions|RotationFromXVector _returnvalue))
  (return (Math|Rotator|MakeRotator (.roll _returnvalue_2) 0.0 (+ (.yaw _returnvalue_2) (Math|Float|SelectFloat 9e+01 -9e+01 (Variables|Spline|GetIs%20Inside%20Spline))))))

(fn GetRotatorfromSplineTangeantwithPointIndex
  (params (Point :type Integer))
  (bind _mysplinecomponent (Variables|Default|GetMySplineComponent))
  (bind _returnvalue (Spline|GetTangentatSplinePoint _mysplinecomponent Point "World"))
  (bind _returnvalue_2 (Math|Conversions|RotationFromXVector _returnvalue))
  (return (Math|Rotator|MakeRotator (.roll _returnvalue_2) 0.0 (+ (.yaw _returnvalue_2) (Math|Float|SelectFloat 9e+01 -9e+01 (Variables|Spline|GetIs%20Inside%20Spline))))))

(fn GetNextPoint
  (params (Current%20Spline%20Point :type Integer) (Stop%20At%20Stop%20Point :type Boolean))
  (bind _returnvalue (+ Current%20Spline%20Point 1))
  (bind _spline_points_count (CallFunction|GetSplinePointCount))
  (if (< _returnvalue (- _spline_points_count 1))
    (for _index (range _returnvalue (- _spline_points_count 1))
      (bind _isstoppoint (Class|MySplineActor|GetPropertyValueatSplinePoint _index))
      (if (== _isstoppoint (Math|Float|SelectFloat 1.0 0.0 Stop%20At%20Stop%20Point))
        (return _index))))
  (return Current%20Spline%20Point))

(fn GetPreviousPoint
  (params (Current%20Spline%20Point :type Integer))
  (bind _spline_points_count (CallFunction|GetSplinePointCount))
  (if (== (- _spline_points_count 1) Current%20Spline%20Point)
    (LocalVariables|Setindex Current%20Spline%20Point)
    (while (>= (LocalVariables|Getindex) 0)
      (bind _isstoppoint (Class|MySplineActor|GetPropertyValueatSplinePoint (LocalVariables|Getindex)))
      (if (== _isstoppoint 0)
        (return 0)
        (else
          (LocalVariables|Setindex (- (LocalVariables|Getindex) 1))))))
  (return Current%20Spline%20Point))