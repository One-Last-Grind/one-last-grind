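; BP_CameraFollowing is a camera actor that classifies where its Target sits along a left-right spline.
; SetActive stores the Target and blends player 0's view to this actor.
; GetLineEquation projects the target onto the XY line through the first two spline points using perpendicular-line intersection, branching for infinite slope, and returns a three-state enum.
; Tick only prints that result; no code here moves the camera.
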(event EventBeginPlay)

(event Collision|EventActorBeginOverlap
  (params (OtherActor :type Actor%20Object%20Reference)))

(event EventTick
  (params (DeltaSeconds :type Float%20%28single-precision%29))
  (Utilities|IsValid (Variables|Default|GetTarget)
    (:Is%20Valid
      (bind _side_on_spline (CallFunction|GetLineEquation))
      (Development|PrintString (Utilities|String|EnumtoString _side_on_spline)))))

(fn ConstructionScript)

(fn SetActive
  (params (Target%20to%20Look :type Actor%20Object%20Reference))
  (Variables|Default|SetTarget Target%20to%20Look)
  (Game|Player|SetViewTargetwithBlend (Game|GetPlayerController 0) self 0.0 "VTBlend_Linear" 0.0 false))

(fn GetLRBounds
  (bind _lr_spline (Variables|Default|GetLR%20Spline))
  (return (Spline|GetLocationatSplinePoint _lr_spline 0 "World") (Spline|GetLocationatSplinePoint _lr_spline 1 "World")))

(fn GetLineEquation
  (bind _target (Variables|Default|GetTarget))
  (bind _returnvalue (Transformation|GetActorLocation _target))
  (bind (_left_bound _right_bound) (CallFunction|GetLRBounds))
  (bind _output_get (LocalVariables|SetLeft%20Bound (Math|Vector|MakeVector (.x _left_bound) (.y _left_bound) 0.0)))
  (bind _output_get_2 (LocalVariables|SetRight%20Bound (Math|Vector|MakeVector (.x _right_bound) (.y _right_bound) 0.0)))
  (if (!= (.x _output_get_2) (.x _output_get))
    ;[0 0 0] Compute Line R Equation Between Right And Left Bounds
    (bind _output_get_3 (LocalVariables|SetMr (/ (- (.y (LocalVariables|GetRight%20Bound)) (.y (LocalVariables|GetLeft%20Bound))) (- (.x (LocalVariables|GetRight%20Bound)) (.x (LocalVariables|GetLeft%20Bound))))))
    (LocalVariables|SetPr (- (.y (LocalVariables|GetLeft%20Bound)) (* _output_get_3 (.x (LocalVariables|GetRight%20Bound)))))
    ;[0 0 0] Compute Orthogonal Line Equation Passing Through The Point Represented By The Target
    (bind _output_get_4 (LocalVariables|SetMs (/ -1.0 (LocalVariables|GetMr))))
    (LocalVariables|SetPs (- (.y _returnvalue) (* _output_get_4 (.x _returnvalue))))
    (if (< (- (/ (.x (- (Math|Vector|MakeVector (/ (- (LocalVariables|GetPs) (LocalVariables|GetPr)) (- (LocalVariables|GetMr) (LocalVariables|GetMs))) (+ (* (LocalVariables|GetMr) (/ (- (LocalVariables|GetPs) (LocalVariables|GetPr)) (- (LocalVariables|GetMr) (LocalVariables|GetMs)))) (LocalVariables|GetPr)) 0.0) (LocalVariables|GetLeft%20Bound))) (.x (- (LocalVariables|GetRight%20Bound) (LocalVariables|GetLeft%20Bound)))) 1.0) 0.0)
      (return "NewEnumerator0")
      (elif (> (- (/ (.x (- (Math|Vector|MakeVector (/ (- (LocalVariables|GetPs) (LocalVariables|GetPr)) (- (LocalVariables|GetMr) (LocalVariables|GetMs))) (+ (* (LocalVariables|GetMr) (/ (- (LocalVariables|GetPs) (LocalVariables|GetPr)) (- (LocalVariables|GetMr) (LocalVariables|GetMs)))) (LocalVariables|GetPr)) 0.0) (LocalVariables|GetLeft%20Bound))) (.x (- (LocalVariables|GetRight%20Bound) (LocalVariables|GetLeft%20Bound)))) 1.0) 1.0)
        (return "NewEnumerator2")
        (else
          (return "NewEnumerator1"))))
    (elif (< (/ (.x (- (Math|Vector|MakeVector (.x (LocalVariables|GetLeft%20Bound)) (.y (Transformation|GetActorLocation (Variables|Default|GetTarget))) 0.0) (LocalVariables|GetLeft%20Bound))) (.x (- (LocalVariables|GetRight%20Bound) (LocalVariables|GetLeft%20Bound)))) 0.0)
      (return "NewEnumerator0")
      (elif (> (/ (.x (- (Math|Vector|MakeVector (.x (LocalVariables|GetLeft%20Bound)) (.y (Transformation|GetActorLocation (Variables|Default|GetTarget))) 0.0) (LocalVariables|GetLeft%20Bound))) (.x (- (LocalVariables|GetRight%20Bound) (LocalVariables|GetLeft%20Bound)))) 1.0)
        (return "NewEnumerator2")
        (else
          (return "NewEnumerator1"))))))