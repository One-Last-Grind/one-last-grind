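; BP_CameraTriggerBox is a trigger that shifts a referenced camera's offset to its target when the third-person character enters it.
; On overlap it stores the current offset and starts a timer.
; Tick then linearly blends to NewCameraOffset over TimeToSwitchOffset, stopping and resetting the timer when done.
; The change is one-way, as leaving the box does not restore the old offset.
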(event EventBeginPlay)

(event Collision|EventActorBeginOverlap
  (params (OtherActor :type Actor%20Object%20Reference))
  (Utilities|Casting|CastToBP_ThirdPersonCharacter OtherActor)
  (Variables|Default|SetIs%20Timer%20Activated true)
  (Variables|Default|SetOld%20Camera%20Offset (Variables|/Game/OneLastGrind/Characters/CameraFollowing/BP_CameraFollowing.BP_CameraFollowing_C|GetCamera%20Offset%20To%20Target (Variables|OLGParameters|GetCamera))))

(event EventTick
  (params (DeltaSeconds :type Float%20%28single-precision%29))
  (if (Variables|Default|GetIs%20Timer%20Activated)
    ;[1 1 1] Timer
    (Variables|Default|SetTimer (+ DeltaSeconds (Variables|Default|GetTimer)))
    (if (Variables|Default|GetIs%20Timer%20Activated)
      (Variables|/Game/OneLastGrind/Characters/CameraFollowing/BP_CameraFollowing.BP_CameraFollowing_C|SetCamera%20Offset%20To%20Target (Variables|OLGParameters|GetCamera) (Math|Float|Lerp (Variables|Default|GetOld%20Camera%20Offset) (Variables|OLGParameters|GetNew%20Camera%20Offset) (Math|Float|MapRangeClamped (Variables|Default|GetTimer) 0.0 (Variables|OLGParameters|GetTime%20To%20Switch%20Offset) 0.0 1.0)))
      (if (>= (Variables|Default|GetTimer) (Variables|OLGParameters|GetTime%20To%20Switch%20Offset))
        (Variables|Default|SetIs%20Timer%20Activated false)
        (Variables|Default|SetTimer 0.0)))))

(fn ConstructionScript)