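; BP_Sphere is a projectile-movement sphere actor, apparently used to test pushing a moving object with impulses.
; Its AddImpulse function adds a force to the current velocity, converts it through the sphere's relative transform and sets it as local-space projectile velocity.
; Tick prints the velocity for debugging.
; A looping timer and a backward push are left unconnected, and its custom event is empty.
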(event Custom|CustomEvent)

(event EventBeginPlay)

(event EventTick
  (params (DeltaSeconds :type Float%20%28single-precision%29))
  (Development|PrintString (Utilities|String|ToString(Vector) (Variables|/Script/Engine.MovementComponent|GetVelocity (Variables|Default|GetProjectileMovement)))))

(fn ConstructionScript
  (Components|Movement|SetUpdatedComponent (Variables|Default|GetProjectileMovement) 0))

(fn AddImpulse
  (params (Force :type Vector))
  (Game|Components|ProjectileMovement|SetVelocityinLocalSpace (Variables|Default|GetProjectileMovement) (Math|Transform|InverseTransformDirection (Transformation|GetRelativeTransform (Variables|Default|GetSphere)) (+ (Transformation|GetVelocity self) Force))))