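; BP_Grindable_SB is a grindable rail actor, built in its Construction Script as either a spline rail or a static mesh with a rail.
; Spline mode tiles clamped-tangent spline meshes by section length and optionally adds pillars between points, scaled down to the ground by line traces.
; Static Mesh mode adds the mesh plus a cylinder spline rail.
; A separate AlignSpline event snaps the spline's end points to a top edge of the mesh bounds.
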(event Custom|AlignSpline
  (bind _spline (Variables|Default|GetSpline))
  (bind _staticmeshcomponent (Variables|Default|GetStaticMeshComponent))
  (bind (_origin _boxextent) (Collision|GetComponentBounds _staticmeshcomponent))
  (bind _returnvalue (* (.x _boxextent) -1.0))
  (switch Utilities|FlowControl|Switch|SwitchonEGrindableType (Variables|Default|GetGrindableType)
    (:NewEnumerator1
      (Spline|SetLocationatSplinePoint _spline 0 (+ _origin (Math|Vector|MakeVector _returnvalue (.y _boxextent) (.z _boxextent))) "World" true)
      (Spline|SetLocationatSplinePoint _spline (- (Spline|GetNumberOfSplinePoints _spline) 1) (+ _origin (Math|Vector|MakeVector _returnvalue (* (.y _boxextent) -1.0) (.z _boxextent))) "World" true))))

(event EventBeginPlay)

(event Collision|EventActorBeginOverlap
  (params (OtherActor :type Actor%20Object%20Reference)))

(event EventTick
  (params (DeltaSeconds :type Float%20%28single-precision%29)))

(fn ConstructionScript
  (switch Utilities|FlowControl|Switch|SwitchonEGrindableType (Variables|Default|GetGrindableType)
    (:NewEnumerator0
      (bind _returnvalue (CallFunction|CreateSplineMesh (Variables|Mesh|GetSplineMesh) (Variables|Mesh|GetSplineMeshMaterial)))
      (if (Variables|Pillars|GetisPillarEnabled)
        (CallFunction|CreatePillars _returnvalue)))
    (:NewEnumerator1
      (CallFunction|CreateSplineMesh "/Game/OneLastGrind/Art/Architecture/S_Cylinder.S_Cylinder" "/Game/OneLastGrind/Art/Materials/GrindableRails/M_GrindableRails.M_GrindableRails")
      (CallFunction|CreateStaticMesh (Variables|Default|GetStatic%20Mesh)))))

(fn CreatePillars
  (params (offSetZ :type Float%20%28double-precision%29))
  (bind _pillarscale (Variables|Pillars|GetpillarScale))
  (for _index (range 0 (- (Spline|GetNumberOfSplinePoints (Variables|Default|GetSpline)) 2))
    (bind _pillarlocation (CallFunction|GetPillarLocation _index "World"))
    (bind _outhit (Collision|LineTraceByChannel _pillarlocation (+ _pillarlocation "0.000000,0.000000,-99999.000000") "TraceTypeQuery1" false 0 "None"))
    (bind _pillarlocation_2 (CallFunction|GetPillarLocation _index "Local"))
    (bind _returnvalue (AddComponent|AddStaticMeshComponent true (Math|Transform|MakeTransform (Math|Vector|MakeVector (.X (Math|Vector|BreakVector _pillarlocation_2)) (.Y (Math|Vector|BreakVector _pillarlocation_2)) (+ (.Z (Math|Vector|BreakVector _pillarlocation_2)) offSetZ)) "0, 0, 0" (Math|Vector|MakeVector _pillarscale _pillarscale (/ (Math|Vector|Distance(Vector) (Math|Vector|MakeVector (.X (Math|Vector|BreakVector _pillarlocation)) (.Y (Math|Vector|BreakVector _pillarlocation)) (+ (.Z (Math|Vector|BreakVector _pillarlocation)) offSetZ)) (.Location (Collision|BreakHitResult _outhit))) -1e+02)))))
    (Components|StaticMesh|SetStaticMesh _returnvalue (Variables|Default|GetPillarMesh))
    (Transformation|AttachComponentToComponent _returnvalue (Variables|Default|GetScene) "None" "KeepRelative" "KeepRelative" "KeepRelative" true)))

(fn GetPillarLocation
  (params (splinePoint :type Integer) (CoordinateSpace :type ESplineCoordinateSpace%20Enum :default "World"))
  (return (Class|SplineComponent|GetLocationatSplineInputKey (Variables|Default|GetSpline) (+ splinePoint 0.5) CoordinateSpace)))

(fn CreateSplineMesh
  (params (SplineStaticMesh :type Static%20Mesh%20Object%20Reference) (Material :type Material%20Interface%20Object%20Reference))
  (bind _spline (Variables|Default|GetSpline))
  (bind _spline_2 (Variables|Default|GetSpline))
  (bind _sectionlength (Variables|Mesh|GetSectionLength))
  (bind _splinemesh (Variables|Mesh|GetSplineMesh))
  (bind _returnvalue (StaticMesh|GetBounds _splinemesh))
  (for _index (range 0 (Math|Float|Truncate (/ (Spline|GetSplineLength (Variables|Default|GetSpline)) (Variables|Mesh|GetSectionLength))))
    (bind _returnvalue_2 (AddComponent|AddSplineMeshComponent true (Math|Transform|MakeTransform (* (.origin _returnvalue) "-1.000000,-1.000000,-1.000000") "0, 0, 0" "1.000000,1.000000,1.000000")))
    (Components|StaticMesh|SetStaticMesh _returnvalue_2 SplineStaticMesh)
    (Rendering|Material|SetMaterial _returnvalue_2 0 Material)
    (SplineMesh|SetForwardAxis _returnvalue_2 (Variables|Mesh|GetSplineMeshForwardAxis) true)
    (Collision|SetCollisionEnabled _returnvalue_2 (Variables|Mesh|GetCollisionTypeEnabled))
    (SplineMesh|SetStartandEnd _returnvalue_2 (Spline|GetLocationatDistanceAlongSpline _spline_2 (* _index _sectionlength) "Local") (Math|Vector|ClampVectorSize (Spline|GetTangentatDistanceAlongSpline _spline_2 (* _index _sectionlength) "Local") 0.0 (Variables|Mesh|GetSectionLength)) (Spline|GetLocationatDistanceAlongSpline _spline (* (+ _index 1) _sectionlength) "Local") (Math|Vector|ClampVectorSize (Spline|GetTangentatDistanceAlongSpline _spline (* (+ _index 1) _sectionlength) "Local") 0.0 (Variables|Mesh|GetSectionLength)) true :!class /Script/Engine.SplineMeshComponent)
    (Transformation|AttachComponentToComponent _returnvalue_2 (Variables|Default|GetScene) "None" "KeepRelative" "KeepRelative" "KeepRelative" true))
  (return (* (.z (.boxextent _returnvalue)) -1.0)))

(fn CreateStaticMesh
  (params (staticMesh :type Static%20Mesh%20Object%20Reference))
  (bind _returnvalue (AddComponent|AddStaticMeshComponent true))
  (bind _output_get (Variables|Default|SetStaticMeshComponent _returnvalue))
  (Components|StaticMesh|SetStaticMesh _output_get staticMesh)
  (Collision|SetCollisionEnabled (Variables|Default|GetStaticMeshComponent) "QueryAndPhysics")
  (Transformation|AttachComponentToComponent (Variables|Default|GetStaticMeshComponent) (Variables|Default|GetScene) "None" "KeepRelative" "KeepRelative" "KeepRelative" true))