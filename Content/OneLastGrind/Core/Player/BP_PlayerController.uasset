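; BP_PlayerController is the player controller for One Last Grind, handling UI and input setup when play begins.
; BeginPlay creates and stores a speed/angle debug widget and flags it as created, without adding it to the viewport here.
; It then registers the IMC_OneLastGrind Enhanced Input mapping context.
; Casts to an old character Blueprint and the game mode are left unconnected.
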(event EventBeginPlay
  (Utilities|FlowControl|Sequence
    (:then_0
      ;[0.4989 0.6383 1] UI Elements
      (bind _returnvalue (UserInterface|CreateWidget "/Game/OneLastGrind/UI/WBP_DebugSpeedAngle.WBP_DebugSpeedAngle_C" self))
      (Variables|Default|SetWBP_Debug _returnvalue)
      (Variables|Default|SetisWidgetDebugCreated true))
    (:then_1
      ;[1 0.4483 0.1218] Input Context
      (Input|AddMappingContext (PlayerController|LocalPlayerSubsystems|GetEnhancedInputLocalPlayerSubsystem self) "/Game/OneLastGrind/Characters/Input/IMC_OneLastGrind.IMC_OneLastGrind" 0 "(bIgnoreAllPressedKeysUntilRelease=True,bForceImmediately=False,bNotifyUserSettings=False)"))))

(fn ConstructionScript)