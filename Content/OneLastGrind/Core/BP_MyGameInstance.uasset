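; Game instance for One Last Grind that loads and applies the player's saved settings at startup.
; Init loads the BP_Settings save slot, or creates and saves one, then applies its parameters and pushes master, music, SFX and voice volumes through sound mix class overrides.
; On first creation, a hardware benchmark sets the scalability levels, which are converted to settings enums and stored as the initial quality values.
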(event EventInit
  (CallFunction|CreateorLoadSettings)
  (Default|ApplyParameters (Variables|Default|GetSettings%20File))
  (Audio|SetSoundMixClassOverride 0 "/Engine/EngineSounds/Master.Master" (Variables|/Game/OneLastGrind/Core/Saves/BP_Settings.BP_Settings_C|GetMaster%20Volume (Variables|Default|GetSettings%20File)) 1.0 1.0 true)
  (Audio|SetSoundMixClassOverride 0 "/Engine/EngineSounds/Music.Music" (Variables|/Game/OneLastGrind/Core/Saves/BP_Settings.BP_Settings_C|GetMusic%20Volume (Variables|Default|GetSettings%20File)) 1.0 1.0 true)
  (Audio|SetSoundMixClassOverride 0 "/Engine/EngineSounds/SFX.SFX" (Variables|/Game/OneLastGrind/Core/Saves/BP_Settings.BP_Settings_C|GetEffect%20Volume (Variables|Default|GetSettings%20File)) 1.0 1.0 true)
  (Audio|SetSoundMixClassOverride 0 "/Engine/EngineSounds/Voice.Voice" (Variables|/Game/OneLastGrind/Core/Saves/BP_Settings.BP_Settings_C|GetVoice%20Volume (Variables|Default|GetSettings%20File)) 1.0 1.0 true)
  (Audio|PushSoundMixModifier 0))

(fn CreateorLoadSettings
  (bind _returnvalue (SaveGame|DoesSaveGameExist (Variables|Default|GetSettings%20Filename)))
  (if _returnvalue
    (bind _returnvalue_2 (SaveGame|LoadGamefromSlot (Variables|Default|GetSettings%20Filename)))
    (bind _asbp_settings (Utilities|Casting|CastToBP_Settings _returnvalue_2))
    (bind _output_get (Variables|Default|SetSettings%20File _asbp_settings))
    (bind _output_get_2 (Variables|/Game/OneLastGrind/Core/Saves/BP_Settings.BP_Settings_C|SetSlot%20Name _output_get (Variables|Default|GetSettings%20Filename)))
    (SaveGame|SaveGametoSlot _output_get _output_get_2)
    (else
      (bind _returnvalue_3 (SaveGame|CreateSaveGameObject "/Game/OneLastGrind/Core/Saves/BP_Settings.BP_Settings_C"))
      (bind _output_get_3 (Variables|Default|SetSettings%20File _returnvalue_3))
      (CallFunction|LoadNewHardwareSettings)
      (bind _output_get_4 (Variables|/Game/OneLastGrind/Core/Saves/BP_Settings.BP_Settings_C|SetSlot%20Name _output_get_3 (Variables|Default|GetSettings%20Filename)))
      (SaveGame|SaveGametoSlot _output_get_3 _output_get_4))))

(fn LoadNewHardwareSettings
  (bind _returnvalue (Settings|GetGameUserSettings))
  (Class|GameUserSettings|RunHardwareBenchmark _returnvalue 10 1.0 1.0)
  (Class|GameUserSettings|ApplyHardwareBenchmarkResults _returnvalue)
  (bind (_texture_quality _anti_aliasing_quality _shadow_quality _visual_effect_quality _shading_quality _view_distance) (CallFunction|GetCurrentSettings))
  (Variables|/Game/OneLastGrind/Core/Saves/BP_Settings.BP_Settings_C|SetTexture%20Quality (Variables|Default|GetSettings%20File) _texture_quality)
  (Variables|/Game/OneLastGrind/Core/Saves/BP_Settings.BP_Settings_C|SetAnti%20Aliasing (Variables|Default|GetSettings%20File) _anti_aliasing_quality)
  (Variables|/Game/OneLastGrind/Core/Saves/BP_Settings.BP_Settings_C|SetShadow%20Quality (Variables|Default|GetSettings%20File) _shadow_quality)
  (Variables|/Game/OneLastGrind/Core/Saves/BP_Settings.BP_Settings_C|SetVFX%20Quality (Variables|Default|GetSettings%20File) _visual_effect_quality)
  (Variables|/Game/OneLastGrind/Core/Saves/BP_Settings.BP_Settings_C|SetShading%20Quality (Variables|Default|GetSettings%20File) _shading_quality)
  (Variables|/Game/OneLastGrind/Core/Saves/BP_Settings.BP_Settings_C|SetView%20Distance (Variables|Default|GetSettings%20File) _view_distance))

(fn GetCurrentSettings
  (bind _returnvalue (Settings|GetGameUserSettings))
  (return (Utilities|Enum|ByteToEnumESettingsLevels (Math|Conversions|ToByte(Integer) (Class|GameUserSettings|GetTextureQuality _returnvalue))) (Utilities|Enum|ByteToEnumESettingsLevels (Math|Conversions|ToByte(Integer) (Class|GameUserSettings|GetAntiAliasingQuality _returnvalue))) (Utilities|Enum|ByteToEnumESettingsLevels (Math|Conversions|ToByte(Integer) (Settings|GetShadowQuality _returnvalue))) (Utilities|Enum|ByteToEnumESettingsLevels (Math|Conversions|ToByte(Integer) (Settings|GetVisualEffectQuality _returnvalue))) (Utilities|Enum|ByteToEnumESettingsLevels (Math|Conversions|ToByte(Integer) (Class|GameUserSettings|GetShadingQuality _returnvalue))) (Utilities|Enum|ByteToEnumESettingsDistances (Math|Conversions|ToByte(Integer) (Class|GameUserSettings|GetViewDistanceQuality _returnvalue)))))