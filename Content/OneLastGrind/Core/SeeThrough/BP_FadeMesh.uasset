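; BP_FadeMesh is a mesh actor that fades toward a partial transparency on request, likely for see-through occluders given its SeeThrough folder.
; The construction script assigns the configured mesh and puts a dynamic instance of FadeMaterial on material slot 0.
; StartFade plays a timeline that drives the material's Opacity parameter from opaque toward EndingFadeAmount, and EndFade reverses it.
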(event EventEndFade
  (bind _fade_amount (Timeline|Fade%20Timeline Reverse)
    (:Update
      (Rendering|Material|SetScalarParameterValue (Variables|Default|GetDynamic%20Material) "Opacity" (- 1.0 (* _fade_amount (- 1.0 (Variables|Default|GetEnding%20Fade%20Amount)))) :!class /Script/Engine.MaterialInstanceDynamic))))

(event EventStartFade
  (bind _fade_amount (Timeline|Fade%20Timeline Play)
    (:Update
      (Rendering|Material|SetScalarParameterValue (Variables|Default|GetDynamic%20Material) "Opacity" (- 1.0 (* _fade_amount (- 1.0 (Variables|Default|GetEnding%20Fade%20Amount)))) :!class /Script/Engine.MaterialInstanceDynamic))))

(fn ConstructionScript
  (Components|StaticMesh|SetStaticMesh (Variables|Default|GetStaticMesh) (Variables|Default|GetMesh%20To%20Use))
  (bind _returnvalue (Rendering|Material|CreateDynamicMaterialInstance (Variables|Default|GetFade%20Material) "None" "None" :!class /Script/Engine.KismetMaterialLibrary))
  (bind _output_get (Variables|Default|SetDynamic%20Material _returnvalue))
  (Rendering|Material|SetMaterial (Variables|Default|GetStaticMesh) 0 _output_get))