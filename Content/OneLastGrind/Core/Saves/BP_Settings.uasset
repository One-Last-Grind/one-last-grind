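; SaveGame object that stores the player's graphics, display and audio volume settings for One Last Grind.
; Each setter writes its value and immediately saves the object to its slot, and grouped getters return the volume, graphics and display values.
; ApplyParameters pushes the quality and display values into GameUserSettings and applies the resolution, but leaves volumes untouched and never calls a full ApplySettings.
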(fn SetTextureQuality
  (params (New%20Value :type ESettingsLevels%20Enum :default "NewEnumerator0"))
  (Variables|Quality|SetTexture%20Quality New%20Value)
  (SaveGame|SaveGametoSlot self (Variables|Default|GetSlot%20Name)))

(fn SetAntiAliasing
  (params (New%20Value :type ESettingsLevels%20Enum :default "NewEnumerator0"))
  (Variables|Quality|SetAnti%20Aliasing New%20Value)
  (SaveGame|SaveGametoSlot self (Variables|Default|GetSlot%20Name)))

(fn SetShadowQuality
  (params (New%20Value :type ESettingsLevels%20Enum :default "NewEnumerator0"))
  (Variables|Quality|SetShadow%20Quality New%20Value)
  (SaveGame|SaveGametoSlot self (Variables|Default|GetSlot%20Name)))

(fn SetShadingQuality
  (params (New%20Value :type ESettingsLevels%20Enum :default "NewEnumerator0"))
  (Variables|Quality|SetShading%20Quality New%20Value)
  (SaveGame|SaveGametoSlot self (Variables|Default|GetSlot%20Name)))

(fn SetVFXQuality
  (params (New%20Value :type ESettingsLevels%20Enum :default "NewEnumerator0"))
  (Variables|Quality|SetVFX%20Quality New%20Value)
  (SaveGame|SaveGametoSlot self (Variables|Default|GetSlot%20Name)))

(fn SetViewDistance
  (params (New%20Value :type ESettingsDistances%20Enum :default "NewEnumerator0"))
  (Variables|Quality|SetView%20Distance New%20Value)
  (SaveGame|SaveGametoSlot self (Variables|Default|GetSlot%20Name)))

(fn SetVSync
  (params (New%20Value :type Boolean))
  (Variables|Display|SetVSync%20On New%20Value)
  (SaveGame|SaveGametoSlot self (Variables|Default|GetSlot%20Name)))

(fn SetResolution
  (params (Resolution :type Int%20Point%20Structure))
  (Variables|Display|SetResolution Resolution)
  (SaveGame|SaveGametoSlot self (Variables|Default|GetSlot%20Name)))

(fn SetDisplayMode
  (params (New%20Value :type EWindowMode%20Enum :default "Fullscreen"))
  (Variables|Display|SetDisplay%20Mode New%20Value)
  (SaveGame|SaveGametoSlot self (Variables|Default|GetSlot%20Name)))

(fn SetMasterVolume
  (params (New%20Volume :type Float%20%28double-precision%29))
  (Variables|Audio|SetMaster%20Volume New%20Volume)
  (SaveGame|SaveGametoSlot self (Variables|Default|GetSlot%20Name)))

(fn SetMusicVolume
  (params (New%20Volume :type Float%20%28double-precision%29))
  (Variables|Audio|SetMusic%20Volume New%20Volume)
  (SaveGame|SaveGametoSlot self (Variables|Default|GetSlot%20Name)))

(fn SetEffectVolume
  (params (New%20Volume :type Float%20%28double-precision%29))
  (Variables|Audio|SetEffect%20Volume New%20Volume)
  (SaveGame|SaveGametoSlot self (Variables|Default|GetSlot%20Name)))

(fn SetVoiceVolume
  (params (New%20Volume :type Float%20%28double-precision%29))
  (Variables|Audio|SetVoice%20Volume New%20Volume)
  (SaveGame|SaveGametoSlot self (Variables|Default|GetSlot%20Name)))

(fn SetFramerateLimit
  (params (New%20Value :type Float%20%28double-precision%29))
  (Variables|Display|SetFramerate%20Limit New%20Value)
  (SaveGame|SaveGametoSlot self (Variables|Default|GetSlot%20Name)))

(fn GetVolumesSettings
  (return (Variables|Audio|GetMaster%20Volume) (Variables|Audio|GetMusic%20Volume) (Variables|Audio|GetEffect%20Volume) (Variables|Audio|GetVoice%20Volume)))

(fn GetGraphicsSettings
  (return (Variables|Quality|GetTexture%20Quality) (Variables|Quality|GetAnti%20Aliasing) (Variables|Quality|GetShadow%20Quality) (Variables|Quality|GetShading%20Quality) (Variables|Quality|GetVFX%20Quality) (Variables|Quality|GetView%20Distance)))

(fn GetDisplaySettings
  (return (Variables|Display|GetVSync%20On) (Variables|Display|GetResolution) (Variables|Display|GetDisplay%20Mode) (Variables|Display|GetFramerate%20Limit)))

(fn ApplyParameters
  (bind _returnvalue (Settings|GetGameUserSettings))
  (Utilities|FlowControl|Sequence
    (:then_0
      (Class|GameUserSettings|SetTextureQuality _returnvalue (Math|Conversions|ToInteger(Byte) (Variables|Quality|GetTexture%20Quality)))
      (Class|GameUserSettings|SetAntiAliasingQuality _returnvalue (Math|Conversions|ToInteger(Byte) (Variables|Quality|GetAnti%20Aliasing)))
      (Class|GameUserSettings|SetShadowQuality _returnvalue (Math|Conversions|ToInteger(Byte) (Variables|Quality|GetShadow%20Quality)))
      (Class|GameUserSettings|SetShadingQuality _returnvalue (Math|Conversions|ToInteger(Byte) (Variables|Quality|GetShading%20Quality)))
      (Class|GameUserSettings|SetVisualEffectQuality _returnvalue (Math|Conversions|ToInteger(Byte) (Variables|Quality|GetVFX%20Quality)))
      (Class|GameUserSettings|SetViewDistanceQuality _returnvalue (Math|Conversions|ToInteger(Byte) (Variables|Quality|GetView%20Distance))))
    (:then_1
      (Class|GameUserSettings|SetScreenResolution _returnvalue (Variables|Display|GetResolution))
      (Class|GameUserSettings|SetFullscreenMode _returnvalue (Variables|Display|GetDisplay%20Mode))
      (Class|GameUserSettings|ApplyResolutionSettings _returnvalue false)
      (Class|GameUserSettings|SetVSyncEnabled _returnvalue (Variables|Display|GetVSync%20On))
      (Class|GameUserSettings|SetFrameRateLimit _returnvalue (Variables|Display|GetFramerate%20Limit)))))