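; BP_SlidingCamera is a placeable trigger that briefly shows a focus point through its own camera.
; On BeginPlay the camera rotates to face the FocusPoint component.
; The first time a BP_TPSNoCamera enters the box, the player's view blends to this actor using eased in-out.
; After the blend-in time plus a hold delay, the view blends back to the camera supplied by that character.
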(event OnComponentBeginOverlap(Box)
  (params (OverlappedComponent :type Primitive%20Component%20Object%20Reference) (OtherActor :type Actor%20Object%20Reference) (OtherComp :type Primitive%20Component%20Object%20Reference) (OtherBodyIndex :type Integer) (bFromSweep :type Boolean) (SweepResult :type Hit%20Result%20Structure%20%28by%20ref%29))
  (bind _asbp_tpsno_camera (Utilities|Casting|CastToBP_TPSNoCamera OtherActor))
  (Utilities|FlowControl|DoOnce false
    (:Completed
      (Game|Player|SetViewTargetwithBlend (Game|GetPlayerController 0) self (Variables|Timers|GetBlend%20Time%20In) "VTBlend_EaseInOut" 3.0 false)
      (Utilities|FlowControl|Delay (+ (Variables|Timers|GetBlend%20Time%20In) (Variables|Timers|GetDelay%20Stop%20Focus)))
      (bind _camera (Default|GetCamera _asbp_tpsno_camera))
      (Game|Player|SetViewTargetwithBlend (Game|GetPlayerController 0) _camera (Variables|Timers|GetBlend%20Time%20Out) "VTBlend_EaseInOut" 3.0 false))))

(event Custom|Set%20Camera%20Position
  (Transformation|SetWorldRotation (Variables|Default|GetCamera) (Math|Rotator|FindLookatRotation (Transformation|GetWorldLocation (Variables|Default|GetCamera)) (Transformation|GetWorldLocation (Variables|Default|GetFocus%20Point))) false false))

(event EventBeginPlay
  (CallFunction|SetCameraPosition))

(fn ConstructionScript
  (Transformation|SetWorldScale3D (Variables|Default|GetFocus%20Point) "0.500000,0.500000,0.500000")
  (Transformation|SetWorldScale3D (Variables|Default|GetCamera) "1.000000,1.000000,1.000000"))